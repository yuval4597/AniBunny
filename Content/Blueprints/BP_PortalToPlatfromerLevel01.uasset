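; Portal actor that sends the player to the PlatformerLevel01 level on overlap, spinning slightly every tick.
; When a BP_PlayerPawn overlaps it, it calls Kill on the pawn after a game instance cast check.
; It then has BP_AniBunnyGameInstance save plant data and the collectible database before opening the level by name.
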(event `self.ReceiveActorBeginOverlap`
  (params (OtherActor :type "Actor Object Reference"))
  (bind _asbp_player_pawn (cast `/Game/Blueprints/BP_PlayerPawn` OtherActor))
  (cast `BAniBunnyGameInstance` (`GameplayStatics.GetGameInstance`))
  (`BCharacter.Kill` _asbp_player_pawn)
  (bind _asbp_ani_bunny_game_instance (cast `/Game/Blueprints/BP_AniBunnyGameInstance` (`GameplayStatics.GetGameInstance`)))
  (`/Game/Blueprints/BP_AniBunnyGameInstance.SavePlantData` _asbp_ani_bunny_game_instance)
  (`/Game/Blueprints/BP_AniBunnyGameInstance.SaveCollectibleDataBase` _asbp_ani_bunny_game_instance)
  (`GameplayStatics.OpenLevel` "PlatformerLevel01"))

(event `self.ReceiveTick`
  (params (DeltaSeconds :type "Float (single-precision)"))
  (`self.K2_AddActorLocalRotation` (struct :`Yaw` 1.0)))

(fn `UserConstructionScript`)