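; Game instance that carries plant and flower collectible state across level switches between the base and platformer worlds.
; Plant saving records each plantable's class, transform and remaining grow time; loading respawns them at unit scale.
; Collectibles are keyed by object name in separate base and platformer maps, storing respawn time or -1 for no respawn.
; Loads subtract time-of-day elapsed since saving from grow and respawn timers, then clear the saved data.
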(fn `LoadCollectibleDataBase`
  (bind _basecollectibletimetorespawn (`self.BaseCollectibleTimeToRespawn`))
  (if (> (`BlueprintMapLibrary.Map_Length` (`self.BaseCollectibleTimeToRespawn`)) 0)
    (bind _outactors (`GameplayStatics.GetAllActorsOfClass` "/Game/Collectibles/BP_FlowerCollectible.BP_FlowerCollectible_C"))
    (for _array_element _outactors
      (bind _timetorespawn (`/Game/Collectibles/BP_FlowerCollectible.TimeToRespawn` _array_element))
      (bind _value (`BlueprintMapLibrary.Map_Find` _basecollectibletimetorespawn (`KismetSystemLibrary.GetObjectName` _array_element)))
      (if (== _timetorespawn _value)
        _
        (elif (== _value -1.0)
          (`/Game/Collectibles/BP_FlowerCollectible.SetInactive` _array_element -1.0)
          (else
            (`/Game/Collectibles/BP_FlowerCollectible.SetInactive` _array_element (`KismetMathLibrary.FClamp` (- _value (`KismetMathLibrary.GetTotalSeconds` (- (`KismetMathLibrary.GetTimeOfDay` (`KismetMathLibrary.Now`)) (`KismetMathLibrary.GetTimeOfDay` (`self.BaseCollectibleSaveWorldTime`))))) 0.1 _timetorespawn))))))
    (`BlueprintMapLibrary.Map_Clear` _basecollectibletimetorespawn)))

(fn `LoadCollectibleDataPlatformer`
  (bind _platformercollectibletimetorespawn (`self.PlatformerCollectibleTimeToRespawn`))
  (if (> (`BlueprintMapLibrary.Map_Length` (`self.PlatformerCollectibleTimeToRespawn`)) 0)
    (bind _outactors (`GameplayStatics.GetAllActorsOfClass` "/Game/Collectibles/BP_FlowerCollectible.BP_FlowerCollectible_C"))
    (for _array_element _outactors
      (bind _timetorespawn (`/Game/Collectibles/BP_FlowerCollectible.TimeToRespawn` _array_element))
      (bind _value (`BlueprintMapLibrary.Map_Find` _platformercollectibletimetorespawn (`KismetSystemLibrary.GetObjectName` _array_element)))
      (if (== _timetorespawn _value)
        _
        (elif (== _value -1.0)
          (`/Game/Collectibles/BP_FlowerCollectible.SetInactive` _array_element -1.0)
          (else
            (`/Game/Collectibles/BP_FlowerCollectible.SetInactive` _array_element (`KismetMathLibrary.FClamp` (- _value (`KismetMathLibrary.GetTotalSeconds` (- (`KismetMathLibrary.GetTimeOfDay` (`KismetMathLibrary.Now`)) (`KismetMathLibrary.GetTimeOfDay` (`self.PlatformerCollectibleSaveWorldTime`))))) 0.1 _timetorespawn))))))
    (`BlueprintMapLibrary.Map_Clear` _platformercollectibletimetorespawn)))

(fn `LoadPlantData`
  (bind _plantgrowtimeremaining (`self.PlantGrowTimeRemaining`))
  (bind _plantlocations (`self.PlantLocations`))
  (bind _plantclasses (`self.PlantClasses`))
  (if (> (`KismetArrayLibrary.Array_Length` _plantclasses) 0)
    (for (_array_element _array_index) _plantclasses
      (bind _returnvalue (`|SpawnActorFromClass` _array_element (`KismetMathLibrary.MakeTransform` (.location (`|GetArrayItem` _plantlocations _array_index)) (.rotation (`|GetArrayItem` _plantlocations _array_index))) "Undefined" "OverrideRootScale" null null))
      (`BPlantable.SetGrowTimeRemaining` _returnvalue (- (`|GetArrayItem` _plantgrowtimeremaining _array_index) (`KismetMathLibrary.GetTotalSeconds` (- (`KismetMathLibrary.GetTimeOfDay` (`KismetMathLibrary.Now`)) (`KismetMathLibrary.GetTimeOfDay` (`self.PlantSaveWorldTime`)))))))
    (`KismetArrayLibrary.Array_Clear` _plantclasses)
    (`KismetArrayLibrary.Array_Clear` _plantlocations)
    (`KismetArrayLibrary.Array_Clear` _plantgrowtimeremaining)))

(fn `SaveCollectibleDataBase`
  (locals (TempObjName :type String) (TempRespawnTime :type "Float (double-precision)"))
  (bind _outactors (`GameplayStatics.GetAllActorsOfClass` "/Game/Collectibles/BP_FlowerCollectible.BP_FlowerCollectible_C"))
  (for _array_element _outactors
    (`|ExecutionSequence`
      (:`then_0`
        (set `local.TempObjName` (`KismetSystemLibrary.GetObjectName` _array_element))
        (if (`/Game/Collectibles/BP_FlowerCollectible.IsActive` _array_element)
          (set `local.TempRespawnTime` (`/Game/Collectibles/BP_FlowerCollectible.TimeToRespawn` _array_element))
          (elif (`/Game/Collectibles/BP_FlowerCollectible.ShouldRespawn` _array_element)
            (set `local.TempRespawnTime` (`KismetSystemLibrary.K2_GetTimerRemainingTime` _array_element "Reactivate"))
            (else
              (set `local.TempRespawnTime` -1.0)))))
      (:`then_1`
        (`BlueprintMapLibrary.Map_Add` (`self.BaseCollectibleTimeToRespawn`) (`local.TempObjName`) (`local.TempRespawnTime`)))))
  (set `self.BaseCollectibleSaveWorldTime` (`KismetMathLibrary.Now`)))

(fn `SaveCollectibleDataPlatformer`
  (locals (TempObjName :type String) (TempRespawnTime :type "Float (double-precision)"))
  (bind _outactors (`GameplayStatics.GetAllActorsOfClass` "/Game/Collectibles/BP_FlowerCollectible.BP_FlowerCollectible_C"))
  (for _array_element _outactors
    (`|ExecutionSequence`
      (:`then_0`
        (set `local.TempObjName` (`KismetSystemLibrary.GetObjectName` _array_element))
        (if (`/Game/Collectibles/BP_FlowerCollectible.IsActive` _array_element)
          (set `local.TempRespawnTime` (`/Game/Collectibles/BP_FlowerCollectible.TimeToRespawn` _array_element))
          (elif (`/Game/Collectibles/BP_FlowerCollectible.ShouldRespawn` _array_element)
            (set `local.TempRespawnTime` (`KismetSystemLibrary.K2_GetTimerRemainingTime` _array_element "Reactivate"))
            (else
              (set `local.TempRespawnTime` -1.0)))))
      (:`then_1`
        (`BlueprintMapLibrary.Map_Add` (`self.PlatformerCollectibleTimeToRespawn`) (`local.TempObjName`) (`local.TempRespawnTime`)))))
  (set `self.PlatformerCollectibleSaveWorldTime` (`KismetMathLibrary.Now`)))

(fn `SavePlantData`
  (`|ExecutionSequence`
    (:`then_0`
      (bind _outactors (`GameplayStatics.GetAllActorsOfClass` "/Script/AniBunny.BPlantable"))
      (for _array_element _outactors
        (`|ExecutionSequence`
          (:`then_0`
            (`KismetArrayLibrary.Array_Add` (`self.PlantClasses`) (`GameplayStatics.GetObjectClass` _array_element)))
          (:`then_1`
            (`KismetArrayLibrary.Array_Add` (`self.PlantLocations`) (`Actor.GetTransform` _array_element)))
          (:`then_2`
            (bind _returnvalue (`BPlantable.GetGrowTimeRemaining` _array_element))
            (`KismetArrayLibrary.Array_Add` (`self.PlantGrowTimeRemaining`) _returnvalue)))))
    (:`then_1`
      (set `self.PlantSaveWorldTime` (`KismetMathLibrary.Now`)))))