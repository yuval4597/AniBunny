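; Base game mode for AniBunny that decides which PlayerStart a player spawns at.
; The ChoosePlayerStart override reads FreshStartTrue from BP_AniBunnyGameInstance, selecting the "FreshStart" tag and clearing the flag, or otherwise the hardcoded "FromPlatfromLevel1" tag.
; It returns the first PlayerStart with that tag, without checking that one exists.
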(fn `ChoosePlayerStart`
  (params (Player :type "Controller Object Reference"))
  (returns (ReturnValue :type "Actor Object Reference"))
  (bind _asbp_ani_bunny_game_instance (cast `/Game/Blueprints/BP_AniBunnyGameInstance` (`GameplayStatics.GetGameInstance`)))
  (`|ExecutionSequence`
    (:`then_0`
      (if (`/Game/Blueprints/BP_AniBunnyGameInstance.FreshStartTrue` _asbp_ani_bunny_game_instance)
        (set `self.PlayerStartTag` "FreshStart")
        (set `/Game/Blueprints/BP_AniBunnyGameInstance.FreshStartTrue` false _asbp_ani_bunny_game_instance)
        (else
          (set `self.PlayerStartTag` "FromPlatfromLevel1"))))
    (:`then_1`
      (bind _outactors (`GameplayStatics.GetAllActorsOfClassWithTag` "/Script/Engine.PlayerStart" (`self.PlayerStartTag`)))
      (return (`|GetArrayItem` _outactors)))))

(fn `UserConstructionScript`)