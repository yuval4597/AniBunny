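; BP_RotatingPlatform is a configurable platform that rotates around a pivot at a set radius.
; The construction script picks a 4x4m or 2m metal box mesh from PlatformType and offsets it along X by Radius.
; The Clockwise flag adjusts RotationRate, which drives the yaw of a RotatingMovement component, so the event graph stays empty.
; An optional PivotObject snaps the actor to that object's location at construction.
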(event `self.ReceiveBeginPlay`)

(event `self.ReceiveTick`
  (params (DeltaSeconds :type "Float (single-precision)")))

(fn `UserConstructionScript`
  (bind _pivotobject (`self.PivotObject`))
  (bind _returnvalue (`KismetMathLibrary.Abs` (`self.RotationRate`)))
  (`|ExecutionSequence`
    (:`then_0`
      (switch `int` (- (`self.PlatformType`) 1)
        (:`Default`
          (`StaticMeshComponent.SetStaticMesh` (`self.PlatformMesh`) "/Game/PlatformerPack/Meshes/Pl_MetalBox_4x4m.Pl_MetalBox_4x4m" :!label _label))
        (:`0`
          (goto _label))
        (:`1`
          (`StaticMeshComponent.SetStaticMesh` (`self.PlatformMesh`) "/Game/PlatformerPack/Meshes/Pl_MetalBox_2m.Pl_MetalBox_2m"))))
    (:`then_1`
      (`SceneComponent.K2_AddLocalOffset` (`self.PlatformMesh`) (`KismetMathLibrary.MakeVector` (`self.Radius`)) false false))
    (:`then_2`
      (if (`self.Clockwise`)
        (set `self.RotationRate` _returnvalue)
        (else
          (bind _result (`/Engine/EditorBlueprintResources/StandardMacros.NegateFloat` _returnvalue)
            (:`  `
              (set `self.RotationRate` _result))))))
    (:`then_3`
      (set `RotatingMovementComponent.RotationRate` (`KismetMathLibrary.MakeRotator` 0.0 0.0 (`self.RotationRate`)) (`self.RotatingMovement`)))
    (:`then_4`
      (`/Engine/EditorBlueprintResources/StandardMacros.IsValid` _pivotobject
        (:`Is Valid`
          (`self.K2_SetActorLocation` (`self.K2_GetActorLocation` _pivotobject) false true))))))