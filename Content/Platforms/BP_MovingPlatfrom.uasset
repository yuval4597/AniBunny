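; Moving platform that oscillates endlessly between two limit points set along local Y.
; The construction script assigns one of two metal box meshes by PlatformType to the platform and both limit components, then offsets the limits by ±Amplitude.
; BeginPlay loops eased MoveComponentTo calls between the limits, with MoveRightFirst choosing the initial direction.
; The first move takes half of Period because it starts midway; each later crossing takes a full Period.
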(event `self.ReceiveBeginPlay`
  (if (`self.MoveRightFirst`)
    (`KismetSystemLibrary.MoveComponentTo` (`self.PlatformMesh`) (`SceneComponent.RelativeLocation` (`self.RightLimit`)) (struct) true true (* (`self.Period`) 0.5))
    (`KismetSystemLibrary.MoveComponentTo` (`self.PlatformMesh`) (`SceneComponent.RelativeLocation` (`self.LeftLimit`)) (struct) true true (`self.Period`) :!label _label)
    (`KismetSystemLibrary.MoveComponentTo` (`self.PlatformMesh`) (`SceneComponent.RelativeLocation` (`self.RightLimit`)) (struct) true true (`self.Period`))
    (goto _label)
    (else
      (`KismetSystemLibrary.MoveComponentTo` (`self.PlatformMesh`) (`SceneComponent.RelativeLocation` (`self.LeftLimit`)) (struct) true true (* (`self.Period`) 0.5))
      (`KismetSystemLibrary.MoveComponentTo` (`self.PlatformMesh`) (`SceneComponent.RelativeLocation` (`self.RightLimit`)) (struct) true true (`self.Period`) :!label _label_2)
      (`KismetSystemLibrary.MoveComponentTo` (`self.PlatformMesh`) (`SceneComponent.RelativeLocation` (`self.LeftLimit`)) (struct) true true (`self.Period`))
      (goto _label_2))))

(fn `UserConstructionScript`
  (`|ExecutionSequence`
    (:`then_0`
      (switch `int` (- (`self.PlatformType`) 1)
        (:`Default`
          (`StaticMeshComponent.SetStaticMesh` (`self.PlatformMesh`) "/Game/PlatformerPack/Meshes/Pl_MetalBox_4x4m.Pl_MetalBox_4x4m" :!label _label)
          (`StaticMeshComponent.SetStaticMesh` (`self.RightLimit`) "/Game/PlatformerPack/Meshes/Pl_MetalBox_4x4m.Pl_MetalBox_4x4m")
          (`StaticMeshComponent.SetStaticMesh` (`self.LeftLimit`) "/Game/PlatformerPack/Meshes/Pl_MetalBox_4x4m.Pl_MetalBox_4x4m"))
        (:`0`
          (goto _label))
        (:`1`
          (`StaticMeshComponent.SetStaticMesh` (`self.PlatformMesh`) "/Game/PlatformerPack/Meshes/Pl_MetalBox_2m.Pl_MetalBox_2m")
          (`StaticMeshComponent.SetStaticMesh` (`self.RightLimit`) "/Game/PlatformerPack/Meshes/Pl_MetalBox_2m.Pl_MetalBox_2m")
          (`StaticMeshComponent.SetStaticMesh` (`self.LeftLimit`) "/Game/PlatformerPack/Meshes/Pl_MetalBox_2m.Pl_MetalBox_2m"))))
    (:`then_1`
      (`SceneComponent.K2_AddLocalOffset` (`self.RightLimit`) (`KismetMathLibrary.MakeVector` 0.0 (`self.Amplitude`)) false false)
      (`SceneComponent.K2_AddLocalOffset` (`self.LeftLimit`) (`KismetMathLibrary.MakeVector` 0.0 (* (`self.Amplitude`) -1.0)) false false))))